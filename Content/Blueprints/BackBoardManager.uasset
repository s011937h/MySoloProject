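; BackBoardManager runs a colour-sequence memory round, with a sequence length set per level.
; Each round rolls a random target combination, then triggers the matching backboard spawner for each colour, one second apart.
; ColourSelected collects picks until the count matches, then CompareCombinations advances or resets the level and starts a new round.
; The comparison checks only the first element of each combination.
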(event `self.ReceiveBeginPlay`
  (`self.BeginNewRound`))

(event `GenerateCombination`
  (for _ (range (`|GetArrayItem` (`self.ColoursPerLevel`) (`self.CurrentLevel`)))
    (`KismetArrayLibrary.Array_Add` (`self.TargetCombination`) (cast `/Game/Blueprints/CombinationColour` (`KismetMathLibrary.Conv_IntToByte` (`KismetMathLibrary.RandomIntegerInRange` 0 (- (enumcount `/Game/Blueprints/CombinationColour`) 1)))))))

(event `BeginNewRound`
  (set `self.Spawned` 0)
  (`KismetArrayLibrary.Array_Clear` (`self.TargetCombination`))
  (`KismetArrayLibrary.Array_Clear` (`self.CurrentCombination`))
  (`self.GenerateCombination`)
  (`KismetSystemLibrary.Delay` 2.0)
  (if (not (== (`self.Spawned`) (`|GetArrayItem` (`self.ColoursPerLevel`) (`self.CurrentLevel`)))) :!label _label
    (`BackBoardSpawn.Spawn` (`|GetArrayItem` (`self.BackBoardSpawners`) (`KismetMathLibrary.Conv_ByteToInt` (`|GetArrayItem` (`self.TargetCombination`) (`self.Spawned`)))))
    (`KismetSystemLibrary.Delay` 1.0)
    (set `self.Spawned` (+ (`self.Spawned`) 1))
    (goto _label)))

(event `ColourSelected`
  (params (Selected :type "/Game/Blueprints/CombinationColour Enum" :default "NewEnumerator0"))
  (bind _currentcombination (`self.CurrentCombination`))
  (`KismetArrayLibrary.Array_Add` _currentcombination Selected)
  (if (== (`KismetArrayLibrary.Array_Length` _currentcombination) (`|GetArrayItem` (`self.ColoursPerLevel`) (`self.CurrentLevel`)))
    (`self.CompareCombinations`)
    (else
      (`KismetSystemLibrary.Delay` 10.0))))

(event `CompareCombinations`
  (set `self.Valid` true)
  (for _ (`self.CurrentCombination`)
    (if (not (`|EnumEquality` (`|GetArrayItem` (`self.TargetCombination`)) (`|GetArrayItem` (`self.CurrentCombination`))))
      (set `self.Valid` false)))
  (if (`self.Valid`)
    (`/Engine/EditorBlueprintResources/StandardMacros.IncrementInt` (`self.CurrentLevel`)
      (:`  `
        _))
    (else
      (set `self.CurrentLevel` 0)))
  (`self.BeginNewRound`))

(fn `UserConstructionScript`)